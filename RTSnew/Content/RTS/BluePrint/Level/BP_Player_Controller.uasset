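; Player controller for an RTS level that turns key presses into commands on the controlled ThirdPersonCharacter.
; W fires the pawn's AttackEvent, and Q calls MoveEvent with the pawn's current location as the target.
; On BeginPlay it shows the mouse cursor and adds the Umg_LAN_test widget to the viewport.
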(event EventBeginPlay
  (Variables|Default|SetbShowMouseCursor true)
  (bind _returnvalue (UserInterface|CreateWidget "/Game/UI/umg_LAN_test.umg_LAN_test_C"))
  (UserInterface|Viewport|AddtoViewport _returnvalue 0))

(event Input|KeyboardEvents|Q
  (params (Key :type Key%20Structure))
  (bind _returnvalue (Pawn|GetControlledPawn))
  (:Pressed
    (bind _asthird_person_character (Utilities|Casting|CastToThirdPersonCharacter _returnvalue))
    (Default|MoveEvent _asthird_person_character (Transformation|GetActorLocation _returnvalue))))

(event Input|KeyboardEvents|W
  (params (Key :type Key%20Structure))
  (:Pressed
    (bind _asthird_person_character (Utilities|Casting|CastToThirdPersonCharacter (Pawn|GetControlledPawn)))
    (Default|AttackEvent _asthird_person_character)))

(fn ConstructionScript)